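; Player pawn for a controllable crane: axis inputs yaw the base boom, pitch two further booms, slide two extensions and adjust camera field of view.
; Rotations step through constant-rate interpolation with clamped pitch, while extensions are clamped to the boom's range.
; Tick holds the inner claw at a fixed world rotation and mutes the audio when all crane inputs are idle.
; BeginPlay records the headset's yaw and resets its orientation and position.
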(event `InputAxis|Pitch1`
  (params (AxisValue :type "Float (single-precision)"))
  (`self.Crane1 Pitch` AxisValue))

(event `InputAxis|Extension`
  (params (AxisValue :type "Float (single-precision)"))
  (`self.Crane Extension` AxisValue))

(event `InputAxis|Pitch2`
  (params (AxisValue :type "Float (single-precision)"))
  (`self.Crane2 Pitch` AxisValue))

(event `InputAxis|Yaw`
  (params (AxisValue :type "Float (single-precision)"))
  (`self.Crane Yaw` AxisValue))

(event `InputAxis|ChangeFieldOfView`
  (params (AxisValue :type "Float (single-precision)"))
  (`CameraComponent.SetFieldOfView` (`self.Camera`) (+ AxisValue (`CameraComponent.FieldOfView` (`self.Camera`)))))

(event `self.ReceiveBeginPlay`
  (set `self.Init Yaw` (.yaw (`HeadMountedDisplayFunctionLibrary.GetOrientationAndPosition`)))
  (`HeadMountedDisplayFunctionLibrary.ResetOrientationAndPosition` 0.0))

(event `self.ReceiveTick`
  (params (DeltaSeconds :type "Float (single-precision)"))
  (`SceneComponent.K2_SetWorldRotation` (`self.Scene_CraneClawInner`) (struct :`Pitch` 180.0) false false)
  (`AudioComponent.SetVolumeMultiplier` (`self.Audio1`) (select `bool` (and (== (`self.GetInputAxisValue`) 0.0) (== (`self.GetInputAxisValue`) 0.0) (== (`self.GetInputAxisValue`) 0.0) (== (`self.GetInputAxisValue`) 0.0)) :`false` 1.0 :!type "Float (single-precision)")))

(event `Crane Yaw`
  (params (Value :type "Float (double-precision)"))
  (`self.Set Relative Rotation` (`self.Scene_CraneBoom0`) (`KismetMathLibrary.MakeRotator` 0.0 0.0 (* Value (`self.AngularSpeed`)))))

(event `Crane1 Pitch`
  (params (Value :type "Float (double-precision)"))
  (bind _scene_craneboom1 (`self.Scene_CraneBoom1`))
  (`self.Set Relative Rotation` _scene_craneboom1 (`KismetMathLibrary.MakeRotator` 0.0 (* Value (`self.AngularSpeed`))))
  (`self.Clamp Angle` _scene_craneboom1 0.0 45.0))

(event `Crane2 Pitch`
  (params (Value :type "Float (double-precision)"))
  (bind _scene_craneboom2 (`self.Scene_CraneBoom2`))
  (`self.Set Relative Rotation` _scene_craneboom2 (`KismetMathLibrary.MakeRotator` 0.0 (* Value (`self.AngularSpeed`))))
  (`self.Clamp Angle` _scene_craneboom2 -80.0 10.0))

(event `Crane Extension`
  (params (value :type "Float (double-precision)"))
  (bind _boomextensionrange (`self.BoomExtensionRange`))
  (bind (_relativelocation_x _relativelocation_y _relativelocation_z) (`KismetMathLibrary.BreakVector` (`SceneComponent.RelativeLocation` (`self.Scene_CraneExtension0`))))
  (bind (_relativelocation_x_2 _relativelocation_y_2 _relativelocation_z_2) (`KismetMathLibrary.BreakVector` (`SceneComponent.RelativeLocation` (`self.Scene_CraneExtension1`))))
  (bind _returnvalue (`KismetMathLibrary.MakeVector` (* value (`self.ExtensionSpeed`))))
  (`SceneComponent.K2_AddLocalOffset` (`self.Scene_CraneExtension0`) _returnvalue false true)
  (`SceneComponent.K2_AddLocalOffset` (`self.Scene_CraneExtension1`) _returnvalue false true)
  (`SceneComponent.K2_SetRelativeLocation` (`self.Scene_CraneExtension0`) (`KismetMathLibrary.MakeVector` (`KismetMathLibrary.FClamp` _relativelocation_x 0.0 _boomextensionrange) _relativelocation_y _relativelocation_z) false true)
  (`SceneComponent.K2_SetRelativeLocation` (`self.Scene_CraneExtension1`) (`KismetMathLibrary.MakeVector` (`KismetMathLibrary.FClamp` _relativelocation_x_2 0.0 _boomextensionrange) _relativelocation_y_2 _relativelocation_z_2) false true))

(fn `UserConstructionScript`)