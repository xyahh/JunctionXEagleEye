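; VR game mode that spawns an old and a new crane pawn and lets the player switch between them.
; On BeginPlay, Init sets a floor tracking origin, spawns both cranes at SpawnHelper actor transforms and calls PossessNext.
; PossessNext cycles player 0 through the pawn array and resets headset orientation and position.
; Tick polls the Tab key, using a DoOnce that resets on release to switch once per press.
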(event `Possess Next`
  (bind _returnvalue (`GameplayStatics.GetPlayerController` 0))
  (`Controller.UnPossess` _returnvalue)
  (set `self.CurrentPawn` (mod (+ (`self.CurrentPawn`) 1) (`KismetArrayLibrary.Array_Length` (`self.Pawns`))))
  (`Controller.Possess` _returnvalue (`|GetArrayItem` (`self.Pawns`) (`self.CurrentPawn`)))
  (`HeadMountedDisplayFunctionLibrary.ResetOrientationAndPosition` 0.0))

(event `self.ReceiveBeginPlay`
  (`self.Init`))

(event `self.ReceiveTick`
  (params (DeltaSeconds :type "Float (single-precision)"))
  (if (`PlayerController.IsInputKeyDown` (`GameplayStatics.GetPlayerController` 0) "Tab")
    (`/Engine/EditorBlueprintResources/StandardMacros.DoOnce` false :!label _label
      (:`Completed`
        (`self.Possess Next`)))
    (else
      (goto _label :!via `Reset`))))

(fn `Init`
  (locals (Spawnhelpers :type "Array of /Game/Blueprints/SpawnHelper Object Reference"))
  (`HeadMountedDisplayFunctionLibrary.SetTrackingOrigin` "Floor")
  (bind _outactors (`GameplayStatics.GetAllActorsOfClass` "/Game/Blueprints/SpawnHelper.SpawnHelper_C"))
  (bind _output_get (set `local.Spawnhelpers` _outactors))
  (bind _returnvalue (`|SpawnActorFromClass` "/Game/Blueprints/NewCranePawn.NewCranePawn_C" (`self.GetTransform` (`|GetArrayItem` _output_get 1)) "AlwaysSpawn" "OverrideRootScale" null null))
  (set `self.NewCrane` _returnvalue)
  (bind _returnvalue_2 (`|SpawnActorFromClass` "/Game/Blueprints/OldCranePawn.OldCranePawn_C" (`self.GetTransform` (`|GetArrayItem` _output_get)) "AlwaysSpawn" "OverrideRootScale" null null))
  (set `self.Old Crane` _returnvalue_2)
  (set `self.Pawns` (`|MakeArray` (`self.Old Crane`) (`self.NewCrane`) :!type "Pawn Object Reference"))
  (`self.Possess Next`))

(fn `UserConstructionScript`)